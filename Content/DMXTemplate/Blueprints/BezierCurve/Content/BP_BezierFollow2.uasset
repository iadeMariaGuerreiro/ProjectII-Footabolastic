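; Actor that loops a sphere along a cubic Bezier curve defined by four point components, with optional debug drawing of the curve.
; While animating, Tick wraps a timer between 0 and 1 to sample the curve and set the sphere's relative location.
; A flag switches sampling and drawing between Blueprint math and external functions.
; The Blueprint math reads world point locations, while the external calls receive relative ones.
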(event EventTick
  (params (DeltaSeconds :type Float%20%28single-precision%29))
  (Utilities|FlowControl|Sequence
    (:then_0
      (if (Variables|Runtime|GetIsAnimating)
        (CallFunction|HandleBezierMovement DeltaSeconds)))
    (:then_1
      (if (Variables|Debug|GetDrawDebugLine)
        (CallFunction|HandleDebugDrawing)))))

(fn ConstructionScript)

(fn SampleBezierCurve
  (params (Time :type Float%20%28double-precision%29))
  (return (+ (* (Math|Float|Power (- 1.0 Time) 3.0) (Transformation|GetWorldLocation (Variables|Default|GetP0))) (* (Math|Float|Power (- 1.0 Time) 2.0) 3.0 Time (Transformation|GetWorldLocation (Variables|Default|GetP1))) (* (- 1.0 Time) (Math|Float|Power Time 2.0) 3.0 (Transformation|GetWorldLocation (Variables|Default|GetP2))) (* (Math|Float|Power Time 3.0) (Transformation|GetWorldLocation (Variables|Default|GetP3))))))

(fn DrawBezier
  (for _index (range 0 (- (Variables|Debug|GetSegments) 1))
    (Rendering|Debug|DrawDebugLine (CallFunction|SampleBezierCurve (Math|Float|SafeDivide (Math|Conversions|ToFloat(Integer) _index) (Math|Conversions|ToFloat(Integer) (Variables|Debug|GetSegments)))) (CallFunction|SampleBezierCurve (Math|Float|SafeDivide (Math|Conversions|ToFloat(Integer) (+ _index 1)) (Math|Conversions|ToFloat(Integer) (Variables|Debug|GetSegments)))) "(R=0.945827,G=0.000000,B=1.000000,A=1.000000)" 0.0 5.0)))

(fn HandleBezierMovement
  (params (DeltaTime :type Float%20%28double-precision%29))
  (|IncrementTimer DeltaTime)
  (if (Variables|Config|GetUseBPVersionOfFunction)
    (Transformation|SetRelativeLocation (Variables|Default|GetSphere) (CallFunction|SampleBezierCurve (Variables|Runtime|GetCurrentTime)) false false)
    (else
      (Transformation|SetRelativeLocation (Variables|Default|GetSphere) (Class|BFLBezierCurve|SampleCubicBezierCurve (Variables|Runtime|GetCurrentTime) (Variables|/Script/Engine.SceneComponent|GetRelativeLocation (Variables|Default|GetP0)) (Variables|/Script/Engine.SceneComponent|GetRelativeLocation (Variables|Default|GetP1)) (Variables|/Script/Engine.SceneComponent|GetRelativeLocation (Variables|Default|GetP2)) (Variables|/Script/Engine.SceneComponent|GetRelativeLocation (Variables|Default|GetP3))) false false))))

(fn HandleDebugDrawing
  (if (Variables|Config|GetUseBPVersionOfFunction)
    (CallFunction|DrawBezier)
    (else
      (Class|BFLBezierCurve|DebugDrawCubicBezierCurve (Variables|Debug|GetSegments) (Variables|/Script/Engine.SceneComponent|GetRelativeLocation (Variables|Default|GetP0)) (Variables|/Script/Engine.SceneComponent|GetRelativeLocation (Variables|Default|GetP1)) (Variables|/Script/Engine.SceneComponent|GetRelativeLocation (Variables|Default|GetP2)) (Variables|/Script/Engine.SceneComponent|GetRelativeLocation (Variables|Default|GetP3)) self "(R=1.000000,G=0.000000,B=0.000000,A=1.000000)" 0.0 3.0))))